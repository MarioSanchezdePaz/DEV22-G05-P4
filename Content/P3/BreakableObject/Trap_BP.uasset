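; Breakable trap actor with a Base held by a physics constraint and cable, apparently meant to drop on enemies.
; The first Box hit sets Activated; only a FirstPersonProjectile then destroys the constraint and detaches the cable end.
; Box overlap waits a second, then applies one-time heavy damage.
; The damage target comes from an unconnected BP_Enemy overlap loop that never runs, so it is never populated.
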(event OnComponentHit(Box)
  (params (HitComponent :type Primitive%20Component%20Object%20Reference) (OtherActor :type Actor%20Object%20Reference) (OtherComp :type Primitive%20Component%20Object%20Reference) (NormalImpulse :type Vector :default "0, 0, 0") (Hit :type Hit%20Result%20Structure%20%28by%20ref%29))
  (if (not (Variables|Default|Getactivated))
    (Variables|Default|Setactivated true)
    (Utilities|Casting|CastToFirstPersonProjectile OtherActor)
    (Components|DestroyComponent (Variables|Default|GetPhysicsConstraint))
    (Physics|AddForce (Variables|Default|Getbase) "0, 0, 0" "None" false)
    (Class|CableComponent|SetAttachEndto (Variables|Default|GetCable) 0 "None" "None")))

(event OnComponentBeginOverlap(Box)
  (params (OverlappedComponent :type Primitive%20Component%20Object%20Reference) (OtherActor :type Actor%20Object%20Reference) (OtherComp :type Primitive%20Component%20Object%20Reference) (OtherBodyIndex :type Integer) (bFromSweep :type Boolean) (SweepResult :type Hit%20Result%20Structure%20%28by%20ref%29))
  (Utilities|FlowControl|Delay 1.0)
  (if (not (Variables|Default|Getused))
    (Game|Damage|ApplyDamage (stale _array_element) 1e+03 0 0)
    (Variables|Default|Setused true)))

(event EventBeginPlay)

(event Collision|EventActorBeginOverlap
  (params (OtherActor :type Actor%20Object%20Reference)))

(event EventTick
  (params (DeltaSeconds :type Float%20%28single-precision%29)))

(fn ConstructionScript)