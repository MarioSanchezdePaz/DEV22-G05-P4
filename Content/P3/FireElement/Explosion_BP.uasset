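; Explosion_BP is a short-lived fire hazard actor that deals continuous damage to actors inside it.
; On BeginPlay it spawns a scaled P_Fire emitter, then removes the emitter and itself after a brief delay.
; FireCollision overlap events maintain the OverlappingActors list.
; Tick damages every listed actor by the truncated Damage value scaled by DeltaSeconds, making Damage a per-second rate.
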(event `self.ReceiveBeginPlay`
  (bind _returnvalue (`GameplayStatics.SpawnEmitterAtLocation` "/Game/StarterContent/Particles/P_Fire.P_Fire" (`self.K2_GetActorLocation`) (struct) (2.0 2.0 1.0)))
  (`KismetSystemLibrary.Delay` 3.0)
  (`ActorComponent.K2_DestroyComponent` _returnvalue)
  (`self.K2_DestroyActor` self))

(event `self.ReceiveTick`
  (params (DeltaSeconds :type "Float (single-precision)"))
  (for _array_element (`self.overlappingActors`)
    (`GameplayStatics.ApplyDamage` _array_element (* (`KismetMathLibrary.FTrunc` (`self.damage`)) DeltaSeconds))))

(event `self.fireCollision.OnComponentBeginOverlap`
  (params (OverlappedComponent :type "PrimitiveComponent Object Reference") (OtherActor :type "Actor Object Reference") (OtherComp :type "PrimitiveComponent Object Reference") (OtherBodyIndex :type Integer) (bFromSweep :type Boolean) (SweepResult :type "HitResult Structure (by ref)"))
  (`KismetArrayLibrary.Array_Add` (`self.overlappingActors`) OtherActor))

(event `self.fireCollision.OnComponentEndOverlap`
  (params (OverlappedComponent :type "PrimitiveComponent Object Reference") (OtherActor :type "Actor Object Reference") (OtherComp :type "PrimitiveComponent Object Reference") (OtherBodyIndex :type Integer))
  (`KismetArrayLibrary.Array_RemoveItem` (`self.overlappingActors`) OtherActor))

(fn `UserConstructionScript`)