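; BP_ShooterEnemy is an AI enemy that fires projectiles and adds 50 health per game instance level on BeginPlay.
; ShootWeapon waits a second, plays a shooting montage, then spawns a projectile offset along its ShooterCamera's rotation with a firing sound.
; AnyDamage reduces health and prints it; at zero, the enemy destroys itself, plays a death sound, sets ImDead and calls EnemyKilled on the player character.
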(event `self.ReceiveBeginPlay`
  (bind _asfirst_person_character (cast `/Game/FirstPersonBP/Blueprints/FirstPersonCharacter` (`GameplayStatics.GetPlayerCharacter` 0)))
  (set `self.FirstPersonInstance` _asfirst_person_character)
  (bind _asmy_game_instance_bp (cast `/Game/P3/MyGameInstance_BP` (`GameplayStatics.GetGameInstance`)))
  (set `self.EnemyHealth` (+ (`KismetMathLibrary.Conv_IntToDouble` (* (`/Game/P3/MyGameInstance_BP.Level` _asmy_game_instance_bp) 50)) (`self.EnemyHealth`))))

(event `ShootWeapon`
  (bind _returnvalue (`SceneComponent.K2_GetComponentRotation` (`self.ShooterCamera`)))
  (`KismetSystemLibrary.Delay` 1.0)
  (`AnimInstance.Montage_Play` (`SkeletalMeshComponent.GetAnimInstance` (`self.Mesh`)) "/Game/P3/AI/Enemy_Mesh_And_Materials/Animation/Shooter/Shooting_AnimationMontage.Shooting_AnimationMontage" 1.0 "MontageLength" 0.0 true)
  (`|SpawnActorFromClass` "/Game/P3/AI/ShooterEnemy/EnemyProjectile.EnemyProjectile_C" (`KismetMathLibrary.MakeTransform` (+ (`SceneComponent.K2_GetComponentLocation` (`self.Projectile`)) (`KismetMathLibrary.GreaterGreater_VectorRotator` (`self.Gun_Offset`) _returnvalue)) _returnvalue) "AdjustIfPossibleButDontSpawnIfColliding" "OverrideRootScale" null null) ; Spawn projectile
  (`GameplayStatics.PlaySoundAtLocation` "/Game/FirstPerson/Audio/FirstPersonTemplateWeaponFire02.FirstPersonTemplateWeaponFire02" (`self.K2_GetActorLocation`) (struct) 0.7 1.0 0.0 null null null) ; Play firing sound
)

(event `self.ReceiveAnyDamage`
  (params (Damage :type "Float (single-precision)") (DamageType :type "DamageType Object Reference") (InstigatedBy :type "Controller Object Reference") (DamageCauser :type "Actor Object Reference"))
  (set `self.EnemyHealth` (- (`self.EnemyHealth`) Damage))
  (if (<= (`self.EnemyHealth`) 0.0)
    (`self.K2_DestroyActor`)
    (`GameplayStatics.PlaySoundAtLocation` "/Game/P3/AI/BasicEnemy/Robot_Death.Robot_Death" (`self.K2_GetActorLocation`) (struct) 1.0 1.0 0.0 null null null)
    (set `self.ImDead` true)
    (bind _asfirst_person_character (cast `/Game/FirstPersonBP/Blueprints/FirstPersonCharacter` (`GameplayStatics.GetPlayerCharacter` 0)))
    (`/Game/FirstPersonBP/Blueprints/FirstPersonCharacter.EnemyKilled` _asfirst_person_character)
    (else
      (`KismetSystemLibrary.PrintString` "Enemy health")
      (`KismetSystemLibrary.PrintString` (`KismetStringLibrary.Conv_DoubleToString` (`self.EnemyHealth`))))))

(fn `UserConstructionScript`)