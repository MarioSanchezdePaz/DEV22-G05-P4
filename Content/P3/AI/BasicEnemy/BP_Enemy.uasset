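; Robot enemy AI character that hunts and attacks the player, with health scaled by game level.
; Pawn sensing sets a Blackboard flag on seeing the player; AttackPlayer sphere-traces ahead to deal damage, then after a delay raises the alarm on all other enemies.
; Low health adds sparks and slows movement, while death spawns an explosion and notifies the player character.
; DeathByGrenade applies fixed damage and reports a kill regardless of remaining health.
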(event `self.ReceiveBeginPlay`
  (set `self.ImDead` false)
  (set `self.MyselfInstance` self)
  (set `self.MyTransform` (`self.GetTransform` self))
  (bind _asmy_game_instance_bp (cast `/Game/P3/MyGameInstance_BP` (`GameplayStatics.GetGameInstance`)))
  (bind _output_get (set `self.EnemyHealth` (+ (`KismetMathLibrary.Conv_IntToDouble` (* (`/Game/P3/MyGameInstance_BP.Level` _asmy_game_instance_bp) 50)) (`self.EnemyHealth`))))
  (`KismetSystemLibrary.PrintString` "Mi vida es ")
  (`KismetSystemLibrary.PrintString` (`KismetStringLibrary.Conv_DoubleToString` _output_get))
  (bind _asfirst_person_character (cast `/Game/FirstPersonBP/Blueprints/FirstPersonCharacter` (`GameplayStatics.GetPlayerCharacter` 0)))
  (set `self.FirstPerson` _asfirst_person_character))

(event `self.PawnSensing.OnSeePawn`
  (params (Pawn :type "Pawn Object Reference"))
  (if (== Pawn (`self.FirstPerson`))
    (`BlackboardComponent.SetValueAsBool` (`AIBlueprintHelperLibrary.GetBlackboard` (`AIBlueprintHelperLibrary.GetAIController` self)) "hasSeenPlayer" true)
    (`KismetSystemLibrary.Delay` 10.0)))

(event `Attack Player`
  (bind _returnvalue (`self.K2_GetActorLocation`))
  (bind (_outhit _returnvalue_2) (`KismetSystemLibrary.SphereTraceSingleForObjects` _returnvalue (+ _returnvalue (* (`KismetMathLibrary.GetForwardVector` (`self.K2_GetActorRotation`)) 250.0)) 120.0 (`|MakeArray` "ObjectTypeQuery3" :!type "EObjectTypeQuery Enum")))
  (if _returnvalue_2
    (bind (_bblockinghit _binitialoverlap _time _distance _location _impactpoint _normal _impactnormal _physmat _hitactor) (`GameplayStatics.BreakHitResult` _outhit))
    (if (and _bblockinghit (== _hitactor (`self.FirstPerson`)))
      (set `self.IsAttacking` true)
      (`KismetSystemLibrary.PrintString` "Attacking!")
      (`GameplayStatics.ApplyDamage` _hitactor 10.0)
      (`KismetSystemLibrary.Delay` 5.0)
      (bind _outactors (`GameplayStatics.GetAllActorsOfClass` "BP_Enemy_C"))
      (for _array_element _outactors
        (if (not (== _array_element (`self.MyselfInstance`)))
          (`self.AlarmActivated` _array_element)))
      (else
        (set `self.IsAttacking` false :!label _label)
        (`KismetSystemLibrary.PrintString` "No ataco")))
    (else
      (goto _label))))

(event `self.ReceiveAnyDamage`
  (params (Damage :type "Float (single-precision)") (DamageType :type "DamageType Object Reference") (InstigatedBy :type "Controller Object Reference") (DamageCauser :type "Actor Object Reference"))
  (bind _returnvalue (`self.GetTransform`))
  (bind _enemyhealth (`self.EnemyHealth`))
  (set `self.EnemyHealth` (- (`self.EnemyHealth`) Damage))
  (if (<= (`self.EnemyHealth`) 0.0)
    (`GameplayStatics.PlaySoundAtLocation` "/Game/P3/AI/BasicEnemy/Robot_Death.Robot_Death" (`self.K2_GetActorLocation`) (struct) 1.0 1.0 0.0 null null null)
    (set `self.ImDead` true)
    (`self.K2_DestroyActor`)
    (bind _asfirst_person_character (cast `/Game/FirstPersonBP/Blueprints/FirstPersonCharacter` (`GameplayStatics.GetPlayerCharacter` 0)))
    (`/Game/FirstPersonBP/Blueprints/FirstPersonCharacter.EnemyKilled` _asfirst_person_character)
    (`|SpawnActorFromClass` "/Game/P3/FireElement/Explosion_BP.Explosion_BP_C" (`KismetMathLibrary.MakeTransform` (`KismetMathLibrary.MakeVector` (.x (.location _returnvalue)) (.y (.location _returnvalue)) (- (.z (.location _returnvalue)) 50.0)) (.rotation _returnvalue) (.scale _returnvalue)) "Undefined" "OverrideRootScale" null null)
    (`KismetSystemLibrary.Delay` 6.0)
    (else
      (`KismetSystemLibrary.PrintString` "Enemy health")
      (`KismetSystemLibrary.PrintString` (`KismetStringLibrary.Conv_DoubleToString` _enemyhealth))
      (if (<= _enemyhealth 50.0)
        (`GameplayStatics.SpawnEmitterAttached` "/Game/StarterContent/Particles/P_Sparks.P_Sparks" (`self.Mesh`))
        (set `CharacterMovementComponent.MaxWalkSpeed` 150.0 (`self.CharacterMovement`))))))

(event `DeathByGrenade`
  (`GameplayStatics.ApplyDamage` self 150.0)
  (bind _asfirst_person_character (cast `/Game/FirstPersonBP/Blueprints/FirstPersonCharacter` (`GameplayStatics.GetPlayerCharacter` 0)))
  (`/Game/FirstPersonBP/Blueprints/FirstPersonCharacter.EnemyKilled` _asfirst_person_character))

(event `AlarmActivated`
  (`BlackboardComponent.SetValueAsBool` (`AIBlueprintHelperLibrary.GetBlackboard` (`AIBlueprintHelperLibrary.GetAIController` self)) "alarmActive" true)
  (`KismetSystemLibrary.PrintString` "Alarma activada"))

(fn `UserConstructionScript`)