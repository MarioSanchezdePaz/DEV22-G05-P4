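; EndGame_BP is an end-of-game trigger actor that spins in the level and finishes play when the first-person character touches it.
; A rotating movement component is added at BeginPlay.
; On collision overlap with FirstPersonCharacter, it shows the WP_EndGame widget with the mouse cursor and UI-only input, removes top-level WP_Health widgets, and pauses the game.
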(event `self.ReceiveBeginPlay`
  (`AddComponent|NODE_AddRotatingMovementComponent-0`))

(event `self.Collision.OnComponentBeginOverlap`
  (params (OverlappedComponent :type "PrimitiveComponent Object Reference") (OtherActor :type "Actor Object Reference") (OtherComp :type "PrimitiveComponent Object Reference") (OtherBodyIndex :type Integer) (bFromSweep :type Boolean) (SweepResult :type "HitResult Structure (by ref)"))
  (bind _returnvalue (`GameplayStatics.GetPlayerController` 0))
  (cast `/Game/FirstPersonBP/Blueprints/FirstPersonCharacter` OtherActor)
  (bind _returnvalue_2 (`|CreateWidget` "/Game/P3/HUD/WP_EndGame.WP_EndGame_C" _returnvalue))
  (`UserWidget.AddToPlayerScreen` _returnvalue_2 0)
  (set `PlayerController.bShowMouseCursor` true _returnvalue)
  (`WidgetBlueprintLibrary.SetInputMode_UIOnlyEx` _returnvalue _returnvalue_2)
  (bind _foundwidgets (`WidgetBlueprintLibrary.GetAllWidgetsOfClass` "/Game/P3/HUD/WP_Health.WP_Health_C"))
  (`Widget.RemoveFromParent` _foundwidgets)
  (`GameplayStatics.SetGamePaused` true))

(fn `UserConstructionScript`)